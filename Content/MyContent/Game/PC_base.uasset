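; Base player controller that routes Enhanced Input actions to the player character and level actors.
; BeginPlay adds the base and light-control mapping contexts at equal priority.
; Input drives jump, crouch, look and control-rotation-relative movement, while the alert and companion-trace actions call AlertLight on BP_RedLight and CastLineTrace on BP_Character's trace component.
; Targets are fetched on each input through GetPlayerCharacter or GetActorOfClass rather than cached references.
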(event Input|EnhancedActionEvents|EnhancedInputActionIA_Crouch
  (params (ActionValue :type Boolean) (ElapsedSeconds :type Float%20%28double-precision%29) (TriggeredSeconds :type Float%20%28double-precision%29) (InputAction :type Input%20Action%20Object%20Reference :default "/Game/MyContent/Inputs/InputActions/PlayerMovement/IA_Crouch.IA_Crouch"))
  (bind _returnvalue (Game|GetPlayerCharacter 0))
  ;[1 1 1] Movement
  (:Started
    (Character|Crouch _returnvalue))
  (:Completed
    (Character|UnCrouch _returnvalue)))

(event Input|EnhancedActionEvents|EnhancedInputActionIA_Jump
  (params (ActionValue :type Boolean) (ElapsedSeconds :type Float%20%28double-precision%29) (TriggeredSeconds :type Float%20%28double-precision%29) (InputAction :type Input%20Action%20Object%20Reference :default "/Game/MyContent/Inputs/InputActions/PlayerMovement/IA_Jump.IA_Jump"))
  (bind _returnvalue (Game|GetPlayerCharacter 0))
  ;[1 1 1] Movement
  (:Started
    (Character|Jump _returnvalue))
  (:Completed
    (Character|StopJumping _returnvalue)))

(event Input|EnhancedActionEvents|EnhancedInputActionIA_Move
  (params (ActionValue :type Vector%202D%20Structure) (ElapsedSeconds :type Float%20%28double-precision%29) (TriggeredSeconds :type Float%20%28double-precision%29) (InputAction :type Input%20Action%20Object%20Reference :default "/Game/MyContent/Inputs/InputActions/PlayerMovement/IA_Move.IA_Move"))
  (bind _returnvalue (Pawn|GetControlRotation :!class /Script/Engine.Controller))
  ;[1 1 1] Movement
  (:Triggered
    (bind _returnvalue_2 (Actor|GetActorOfClass "/Game/MyContent/BP/BP_Character.BP_Character_C"))
    (Pawn|Input|AddMovementInput _returnvalue_2 (Math|Vector|GetRightVector (Math|Rotator|MakeRotator (.roll _returnvalue) 0.0 (.yaw _returnvalue))) (.x ActionValue) false)
    (Pawn|Input|AddMovementInput _returnvalue_2 (Math|Vector|GetForwardVector (Math|Rotator|MakeRotator 0.0 0.0 (.yaw _returnvalue))) (.y ActionValue) false)))

(event Input|EnhancedActionEvents|EnhancedInputActionIA_Alert
  (params (ActionValue :type Boolean) (ElapsedSeconds :type Float%20%28double-precision%29) (TriggeredSeconds :type Float%20%28double-precision%29) (InputAction :type Input%20Action%20Object%20Reference :default "/Game/MyContent/Inputs/InputActions/LightControl/IA_Alert.IA_Alert"))
  ;[1 1 1] Lights control
  (:Started
    (bind _returnvalue (Actor|GetActorOfClass "/Game/MyContent/BP/BP_RedLight.BP_RedLight_C"))
    (Default|AlertLight _returnvalue)))

(event Input|EnhancedActionEvents|EnhancedInputActionIA_Look
  (params (ActionValue :type Vector%202D%20Structure) (ElapsedSeconds :type Float%20%28double-precision%29) (TriggeredSeconds :type Float%20%28double-precision%29) (InputAction :type Input%20Action%20Object%20Reference :default "/Game/MyContent/Inputs/InputActions/PlayerMovement/IA_Look.IA_Look"))
  ;[1 1 1] Camera control
  (:Triggered
    (Class|PlayerController|AddYawInput (.x ActionValue))
    (Class|PlayerController|AddPitchInput (.y ActionValue))))

(event Input|EnhancedActionEvents|EnhancedInputActionIA_CompanionTrace
  (params (ActionValue :type Boolean) (ElapsedSeconds :type Float%20%28double-precision%29) (TriggeredSeconds :type Float%20%28double-precision%29) (InputAction :type Input%20Action%20Object%20Reference :default "/Game/MyContent/Inputs/InputActions/Companion_actions/IA_CompanionTrace.IA_CompanionTrace"))
  ;[1 1 1] Cast LineTrace
  (:Started
    (bind _returnvalue (Actor|GetActorOfClass "/Game/MyContent/BP/BP_Character.BP_Character_C"))
    (Default|CastLineTrace (Variables|/Game/MyContent/BP/BP_Character.BP_Character_C|GetBP_LineTrace_Component _returnvalue))))

(event EventBeginPlay
  (bind _self self)
  (bind _returnvalue (PlayerController|LocalPlayerSubsystems|GetEnhancedInputLocalPlayerSubsystem _self))
  ;[1 1 1] Setting up mapping contexts
  (Utilities|IsValid _returnvalue
    (:Is%20Valid
      (Input|AddMappingContext _returnvalue "/Game/MyContent/Inputs/InputMappings/IMC_base.IMC_base" 0 "(bIgnoreAllPressedKeysUntilRelease=True,bForceImmediately=False)")
      (Input|AddMappingContext _returnvalue "/Game/MyContent/Inputs/InputMappings/IMC_LightControl.IMC_LightControl" 0 "(bIgnoreAllPressedKeysUntilRelease=True,bForceImmediately=False)"))))

(fn ConstructionScript)