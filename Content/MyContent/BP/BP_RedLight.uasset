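; BP_RedLight is a spotlight Blueprint that fades to red when AlertLight is triggered, then returns to white.
; AlertLight steps LerpAlpha up in a Delay loop, setting the SpotLight color by linear color interpolation until fully red.
; A timer holds the red briefly, then fires TurnBackToWhite, which steps the same alpha down more gradually to fade back to white.
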(event Custom|AlertLight
  ;[1 1 1] Change color to red
  (Rendering|Components|Light|SetLightColor (Variables|Default|GetSpotLight) (Math|Color|Lerp(LinearColor) "(R=1.000000,G=1.000000,B=1.000000,A=1.000000)" "(R=1.000000,G=0.000000,B=0.000000,A=1.000000)" (Variables|Default|GetLerp%20alpha)) true :!label _label)
  (Utilities|FlowControl|Delay 0.1)
  (if (>= (Variables|Default|GetLerp%20alpha) 1.0)
    ;[1 1 1] Let the light sit as red for 3s
    (Utilities|Time|SetTimerbyEvent (delegate Custom|TurnBackToWhite) 3.0)
    (else
      (Variables|Default|SetLerp%20alpha (+ (Variables|Default|GetLerp%20alpha) 0.12))
      (goto _label))))

(event Custom|TurnBackToWhite
  ;[1 1 1] Change color back to white
  (Rendering|Components|Light|SetLightColor (Variables|Default|GetSpotLight) (Math|Color|Lerp(LinearColor) "(R=1.000000,G=1.000000,B=1.000000,A=1.000000)" "(R=1.000000,G=0.000000,B=0.000000,A=1.000000)" (Variables|Default|GetLerp%20alpha)) true :!label _label)
  (Utilities|FlowControl|Delay 0.1)
  (if (not (<= (Variables|Default|GetLerp%20alpha) 0.0))
    (Variables|Default|SetLerp%20alpha (- (Variables|Default|GetLerp%20alpha) 0.05))
    (goto _label)))

(fn ConstructionScript)