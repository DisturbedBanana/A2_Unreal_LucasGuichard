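; Surveillance camera actor that turns to follow BP_Character while it overlaps the actor, then eases back to its starting rotation.
; Begin and end overlaps toggle tracking, re-setting looping timers that RInterp the camera toward a look-at rotation with axis offsets or toward the rotation cached at BeginPlay.
; A self-restarting timeline blinks the light material between white and red during tracking, and another fades it from red to white on exit.
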(event Custom|SwitchCameTrackingON/OFF
  (params (loop :type Boolean))
  (Utilities|Time|SetTimerbyEvent (delegate Custom|TrackPlayer) 0.01 loop))

(event Custom|TrackPlayer
  (bind _returnvalue (Utilities|Time|GetWorldDeltaSeconds))
  (bind _player (Variables|Default|Getplayer))
  (bind _surveillancecam (Variables|Default|GetsurveillanceCam))
  (bind _surveillancecam_2 (Variables|Default|GetsurveillanceCam))
  (bind _returnvalue_2 (Transformation|GetActorLocation _player))
  (bind _returnvalue_3 (Transformation|GetWorldLocation _surveillancecam))
  (bind _returnvalue_4 (Transformation|GetWorldRotation _surveillancecam_2))
  (bind _returnvalue_5 (Math|Rotator|FindLookatRotation _returnvalue_3 _returnvalue_2))
  (bind _returnvalue_6 (+ (.yaw _returnvalue_5) -9e+01))
  (bind _returnvalue_7 (* (.pitch _returnvalue_5) -1.0))
  (bind _returnvalue_8 (+ _returnvalue_7 -1e+01))
  (bind _returnvalue_9 (Math|Interpolation|RInterpTo _returnvalue_4 (Math|Rotator|MakeRotator _returnvalue_8 (.roll _returnvalue_5) _returnvalue_6) _returnvalue 3.5))
  (Transformation|SetWorldRotation (Variables|Default|GetsurveillanceCam) (Math|Rotator|MakeRotator (.roll _returnvalue_9) (.pitch _returnvalue_9) (.yaw _returnvalue_9)) false false))

(event Custom|ResetCamPos
  (Transformation|SetWorldRotation (Variables|Default|GetsurveillanceCam) (Math|Interpolation|RInterpTo (Transformation|GetWorldRotation (Variables|Default|GetsurveillanceCam)) (Variables|Default|GetCachedRotation) (Utilities|Time|GetWorldDeltaSeconds) 5.0) false false))

(event Custom|BlinkCameraLight
  (Timeline|Timeline Play
    (:Update
      (if (Variables|Default|GetlightBool)
        (Rendering|Material|SetVectorParameterValueonMaterials (Variables|Default|GetcamLight) "Color" (Math|Conversions|ToVector(LinearColor) (Math|Color|Lerp(LinearColor) "(R=1.000000,G=1.000000,B=1.000000,A=1.000000)" "(R=1.000000,G=0.000000,B=0.000000,A=1.000000)" 0.0)))
        (else
          (Rendering|Material|SetVectorParameterValueonMaterials (Variables|Default|GetcamLight) "Color" (Math|Conversions|ToVector(LinearColor) (Math|Color|Lerp(LinearColor) "(R=1.000000,G=0.000000,B=0.000000,A=1.000000)" "(R=1.000000,G=1.000000,B=1.000000,A=1.000000)" 0.0))))))
    (:Finished
      (Variables|Default|SetlightBool (not (Variables|Default|GetlightBool)))
      (if (Variables|Default|GetshouldTrackPlayer)
        (Timeline|Timeline PlayFromStart)))))

(event Custom|LightBackToWhite
  (bind _track (Timeline|Timeline_0 PlayFromStart)
    (:Update
      (Rendering|Material|SetVectorParameterValueonMaterials (Variables|Default|GetcamLight) "Color" (Math|Conversions|ToVector(LinearColor) (Math|Color|Lerp(LinearColor) "(R=1.000000,G=0.000000,B=0.000000,A=1.000000)" "(R=1.000000,G=1.000000,B=1.000000,A=1.000000)" _track))))))

(event EventBeginPlay
  (bind _returnvalue (Actor|GetActorOfClass "/Game/MyContent/BP/BP_Character.BP_Character_C"))
  (Variables|Default|SetPlayer _returnvalue)
  (Variables|Default|SetCachedRotation (Transformation|GetWorldRotation (Variables|Default|GetsurveillanceCam))))

(event Collision|EventActorBeginOverlap
  (params (OtherActor :type Actor%20Object%20Reference))
  (Utilities|Casting|CastToBP_Character OtherActor)
  (bind _output_get (Variables|Default|SetshouldTrackPlayer (not (Variables|Default|GetshouldTrackPlayer))))
  (CallFunction|SwitchCameTrackingON/OFF _output_get)
  (Utilities|Time|SetTimerbyEvent (delegate Custom|ResetCamPos) 0.1 (not (Variables|Default|GetshouldTrackPlayer)))
  (CallFunction|BlinkCameraLight))

(event Collision|EventActorEndOverlap
  (params (OtherActor :type Actor%20Object%20Reference))
  (Utilities|Casting|CastToBP_Character OtherActor
    (:then
      (bind _output_get (Variables|Default|SetshouldTrackPlayer (not (Variables|Default|GetshouldTrackPlayer))))
      (CallFunction|SwitchCameTrackingON/OFF _output_get)
      (Utilities|Time|SetTimerbyEvent (delegate Custom|ResetCamPos) 0.1 (not (Variables|Default|GetshouldTrackPlayer)))
      (CallFunction|LightBacktoWhite))
    (:CastFailed
      (Development|PrintString "failed"))))

(fn ConstructionScript)