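; BP_LineTrace_Component is a component that casts debug-drawn multi line traces from its owner's location.
; CastLineTrace uses DirectionDecider to pick one of four helpers that set the trace end from the owner's forward, right, backward or left vector.
; The end is the scaled vector without the start location added.
; The DirectionDecider increment is unconnected, so the direction never cycles here, and the hit loop does nothing.
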(event Custom|CastLineTrace
  (bind _output_get (Variables|Default|SetPlayer (Components|GetOwner)))
  (Variables|Default|SetStartLineTraceLocation (Transformation|GetActorLocation _output_get))
  (if (<= (Variables|Default|GetDirection%20Decider) 3)
    _
    (else
      (Variables|Default|SetDirection%20Decider 0)))
  (switch int (Variables|Default|GetDirection%20Decider)
    (:0
      (|TraceGoesForward))
    (:1
      (|TraceGoesRight))
    (:2
      (|TraceGoesBehind))
    (:3
      (|TraceGoesLeft)))
  (bind _outhits (Collision|MultiLineTraceByChannel (Variables|Default|GetStartLineTraceLocation) (Variables|Default|GetEndLineTraceLocation) "TraceTypeQuery3" false 0 "ForDuration"))
  (for _array_element _outhits
    _))