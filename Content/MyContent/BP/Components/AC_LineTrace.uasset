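; Actor component that runs debug-drawn traces for the player character and turrets.
; CastLineTrace multi-traces from the character's Head socket to its scaled forward vector (not offset from the start), calling InteractMessage on BP_Interface turrets and launching other interface actors' meshes upward.
; TurretShoot sphere-traces from the owning turret's "turretgun" mesh, found by name, to the supplied PlayerDir point and only prints when it hits the player.
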(event Custom|CastLineTrace
  ;[1 1 1] Declare Player
  (bind _asbp_character (Utilities|Casting|CastToBP_Character (Components|GetOwner)))
  (bind _output_get (Variables|Default|SetPlayer _asbp_character))
  ;[1 1 1] Start Trace start at companion location - (2 meshes in character so we determine which is companion by checking display name in editor)
  (Variables|Default|SetStartLineTraceLocation (Transformation|GetSocketLocation (Actor|GetComponentbyClass _output_get "/Script/Engine.SkeletalMeshComponent") "Head"))
  ;[1 1 1] Determine where Trace end should be - (here we simply multiply the player's forward vector to get a point in front of it)
  (Variables|Default|SetEndLineTraceLocation (* (Transformation|GetActorForwardVector (Variables|Default|GetPlayer)) (Variables|Default|GetEndDistanceMultiplier)))
  ;[1 1 1] Cast trace and display name of actors hit
  (bind _outhits (Collision|MultiLineTraceByChannel (Variables|Default|GetStartLineTraceLocation) (Variables|Default|GetEndLineTraceLocation) "TraceTypeQuery3" false 0 "ForDuration"))
  (for _array_element _outhits
    ;;[1 1 1] Check if hit object has interface
    (if (Utilities|DoesObjectImplementInterface (.HitActor (Collision|BreakHitResult _array_element)) "/Game/MyContent/BP/BP_Interface.BP_Interface_C")
      ;;[1 1 1] Display Actor name in debug
      (Development|PrintString (Utilities|GetDisplayName (.HitActor (Collision|BreakHitResult _array_element))))
      (Utilities|Casting|CastToBP_Turret (.HitActor (Collision|BreakHitResult _array_element))
        (:then
          (Class|BPInterface|Interact(Message) (.HitActor (Collision|BreakHitResult _array_element))))
        (:CastFailed
          ;;[1 1 1] Get the Actor's mesh to apply an impulse to send it flying when hit
          (Physics|AddImpulse (Actor|GetComponentbyClass (.HitActor (Collision|BreakHitResult _array_element)) "/Script/Engine.StaticMeshComponent") "0.000000,0.000000,10000.000000" "None" false))))))

(event Custom|TurretShoot
  (params (playerDir :type Vector))
  (Variables|Default|SetEndLineTraceLocation playerDir)
  (bind _asbp_turret (Utilities|Casting|CastToBP_Turret (Components|GetOwner)))
  (bind _output_get (Variables|Default|Setturret _asbp_turret))
  (for _array_element (Actor|GetComponentsByClass _output_get "/Script/Engine.StaticMeshComponent")
    (if (Utilities|Enum|Equal(Enum) (Utilities|GetObjectName _array_element) "turretgun")
      (Variables|Default|SetStartLineTraceLocation (Transformation|GetWorldLocation _array_element))
      (bind _outhit (Collision|SphereTraceByChannel (Variables|Default|GetStartLineTraceLocation) (Variables|Default|GetEndLineTraceLocation) 0.0 "TraceTypeQuery4" false 0 "ForDuration" true "(R=1.000000,G=0.000000,B=0.843322,A=1.000000)"))
      (Utilities|Casting|CastToBP_Character (.HitActor (Collision|BreakHitResult _outhit)))
      (Development|PrintString "hit player"))))